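; Player pawn Blueprint that draws a rope effect between the pawn and its launched hook.
; Each Tick sets the Niagara FXRope component's RopeCreated flag from whether LaunchedHook is valid.
; While the hook exists, it also passes the hook's location as the rope start and the pawn's as the target.
; Unconnected rope-rotation and debug-print nodes remain, and the construction script is empty.
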(event EventTick
  (params (DeltaSeconds :type Float%20%28single-precision%29))
  (bind _launchedhook (Variables|Default|GetLaunchedHook))
  (bind _fx_rope (Variables|Default|GetFX_Rope))
  (bind _returnvalue (Utilities|IsValid _launchedhook))
  (Class|NiagaraComponent|SetVariableBool (Variables|Default|GetFX_Rope) "RopeCreated" _returnvalue)
  (if _returnvalue
    (Niagara|SetNiagaraVariable(Vector3) _fx_rope "RopeStart" (Transformation|GetActorLocation _launchedhook))
    (Niagara|SetNiagaraVariable(Vector3) _fx_rope "RopeTarget" (Transformation|GetActorLocation))))

(fn ConstructionScript)