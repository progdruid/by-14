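; BP_FinalArea is an area actor that fades the music volume when a LevelPawn enters or leaves it.
; On BeginPlay it caches the AudioComponent from the referenced MusicActor.
; Begin overlap plays a Timeline whose Volume track drives that component's volume multiplier, and end overlap reverses it.
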(event Collision|EventActorBeginOverlap
  (params (OtherActor :type Actor%20Object%20Reference))
  (if (Utilities|ClassIsChildOf (Utilities|GetClass OtherActor) "/Script/by14.LevelPawn")
    (bind _volume (Timeline|Timeline Play)
      (:Update
        (Audio|Components|Audio|SetVolumeMultiplier (Variables|Default|GetMusic%20Audio%20Component) _volume :!class /Script/Engine.AudioComponent)))))

(event Collision|EventActorEndOverlap
  (params (OtherActor :type Actor%20Object%20Reference))
  (if (Utilities|ClassIsChildOf (Utilities|GetClass OtherActor) "/Script/by14.LevelPawn")
    (bind _volume (Timeline|Timeline Reverse)
      (:Update
        (Audio|Components|Audio|SetVolumeMultiplier (Variables|Default|GetMusic%20Audio%20Component) _volume :!class /Script/Engine.AudioComponent)))))

(event EventBeginPlay
  (Variables|Default|SetMusic%20Audio%20Component (Actor|GetComponentbyClass (Variables|Default|GetMusic%20Actor) "/Script/Engine.AudioComponent")))

(fn ConstructionScript)